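; Game mode for a wave-based enemy game that spawns waves, counts kills and saves the best run.
; Once the game starts, Tick watches for zero living enemies and, through a DoOnce with delayed reset, has every Spawner spawn the next wave's count.
; After the fifteenth wave it shows the DeadScreen widget instead.
; ShoudSave compares kills against save slot "1", saves higher scores and returns the best kills and wave.
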(event Custom|NextWave
  (bind _numofwave (Variables|Default|GetNumOfWave))
  (if (Variables|Default|GetGameStarted)
    (if (>= (Variables|Default|GetNumOfWave) 15)
      (CallFunction|ShowDeadScreen)
      (else
        (bind _outactors (Actor|GetAllActorsOfClass "/Game/Blueprints/Actors/Spawner.Spawner_C"))
        (for _array_element _outactors
          (Default|SpawnEnemy _array_element (Utilities|Array|Get(acopy) (Variables|Default|GetNumOfEnemy) (Variables|Default|GetNumOfWave))))
        (Math|Integer|IncrementInt (Variables|Default|GetNumOfWave)
          (:%20%20
            (Development|PrintString (Utilities|String|Append "NumOfNextWave: " (Utilities|String|ToString(Integer) _numofwave) " 
NextNumOfEnemy: " (Utilities|String|ToString(Integer) (Utilities|Array|Get(acopy) (Variables|Default|GetNumOfEnemy) _numofwave))) true false "(R=1.000000,G=0.843744,B=0.000000,A=1.000000)")))))))

(event Custom|ShowDeadScreen
  (bind _returnvalue (UserInterface|CreateWidget "/Game/Blueprints/Widgets/DeadScreen.DeadScreen_C"))
  (UserInterface|Viewport|AddtoViewport _returnvalue 0)
  (Default|DeadLog _returnvalue))

(event Custom|CountEnemy
  (Math|Integer|IncrementInt (Variables|Default|GetKilledEnemy)))

(event EventBeginPlay
  (bind _returnvalue (SaveGame|CreateSaveGameObject "/Game/Blueprints/SaveInfo.SaveInfo_C"))
  (Variables|Default|SetSaveVariable _returnvalue))

(event EventTick
  (params (DeltaSeconds :type Float%20%28single-precision%29))
  (Development|PrintString (Utilities|String|ToString(Integer) (Variables|Default|GetKilledEnemy)) true false "(R=0.000000,G=0.660000,B=1.000000,A=1.000000)" 0.0)
  (if (Variables|Default|GetGameStarted)
    (bind _outactors (Actor|GetAllActorsOfClass "/Game/Blueprints/EnemyCharacter/EnemyCharacterFather.EnemyCharacterFather_C"))
    (if (< (Utilities|Array|LastIndex _outactors) 0)
      (Utilities|FlowControl|DoOnce false :!label _label
        (:Completed
          (CallFunction|NextWave)
          (Utilities|FlowControl|Delay 2.0)
          (goto _label Reset))))))

(fn ConstructionScript)

(fn ShoudSave
  (bind _killedenemy (Variables|Default|GetKilledEnemy))
  (bind _numofwave (Variables|Default|GetNumOfWave))
  (bind _savevariable (Variables|Default|GetSaveVariable))
  (bind _killedenemy_2 (Variables|Default|GetKilledEnemy))
  (bind _numofwave_2 (Variables|Default|GetNumOfWave))
  (bind _returnvalue (- _numofwave_2 1))
  (bind _returnvalue_2 (- _numofwave 1))
  (Utilities|IsValid _savevariable
    (:Is%20Valid
      (bind _returnvalue_3 (SaveGame|DoesSaveGameExist "1"))
      (if _returnvalue_3
        (bind _returnvalue_4 (SaveGame|LoadGamefromSlot "1"))
        (bind _assave_info (Utilities|Casting|CastToSaveInfo _returnvalue_4))
        (Development|PrintString (Utilities|String|ToString(Integer) (Variables|/Game/Blueprints/SaveInfo.SaveInfo_C|GetNumOfEnemy _assave_info)))
        (if (>= (Variables|/Game/Blueprints/SaveInfo.SaveInfo_C|GetNumOfEnemy _assave_info) (Variables|Default|GetKilledEnemy))
          (return (Variables|/Game/Blueprints/SaveInfo.SaveInfo_C|GetNumOfEnemy _assave_info) (Variables|/Game/Blueprints/SaveInfo.SaveInfo_C|GetNumOfWave _assave_info))
          (else
            (Default|SaveGame _savevariable _killedenemy _returnvalue_2)
            (return _killedenemy _returnvalue_2)))
        (else
          (Default|SaveGame _savevariable _killedenemy_2 _returnvalue)
          (return _killedenemy_2 _returnvalue))))))