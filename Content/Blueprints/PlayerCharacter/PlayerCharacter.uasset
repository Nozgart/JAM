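; Player character Blueprint that tracks health and switches between an action camera and a logic camera.
; Incoming damage lowers Health, and at zero or below it asks MainGameMode to show the dead screen.
; PausedCamera and ResumeCamera events swap which camera component is active.
; Tick prints the current Health on screen as a readout.
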(event Custom|PausedCamera
  (Components|Activation|Deactivate (Variables|Default|GetActionCamera))
  (Components|Activation|Activate (Variables|Default|GetLogicCamera) false))

(event Custom|ResumeCamera
  (Components|Activation|Deactivate (Variables|Default|GetLogicCamera))
  (Components|Activation|Activate (Variables|Default|GetActionCamera) false))

(event EventBeginPlay)

(event Collision|EventActorBeginOverlap
  (params (OtherActor :type Actor%20Object%20Reference)))

(event EventTick
  (params (DeltaSeconds :type Float%20%28single-precision%29))
  (Development|PrintString (Utilities|String|ToString(Float) (Variables|Default|GetHealth)) true false "(R=0.000000,G=0.660000,B=1.000000,A=1.000000)" 0.0))

(event Game|Damage|EventAnyDamage
  (params (Damage :type Float%20%28single-precision%29) (DamageType :type Damage%20Type%20Object%20Reference) (InstigatedBy :type Controller%20Object%20Reference) (DamageCauser :type Actor%20Object%20Reference))
  (bind _output_get (Variables|Default|SetHealth (- (Variables|Default|GetHealth) Damage)))
  (if (<= _output_get 0.0)
    (bind _asmain_game_mode (Utilities|Casting|CastToMainGameMode (Game|GetGameMode)))
    (Default|ShowDeadScreen _asmain_game_mode)))

(event EventDestroyed)

(fn ConstructionScript)