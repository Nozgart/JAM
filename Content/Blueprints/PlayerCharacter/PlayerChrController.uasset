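; Player controller for a top-down shooter character that moves on the ground plane, aims with the visible mouse cursor and shoots.
; Axis input moves the pawn along control-yaw directions, while Tick traces under the cursor to turn PlayerCharacter toward the hit point.
; Shoot briefly raises the character's Attacking flag; a separate Atack event, not called here, spawns a scaled-down Bullet at its Arrow1 transform.
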(event EventTick
  (params (DeltaSeconds :type Float%20%28single-precision%29))
  (bind (_hitresult _returnvalue) (Game|Player|GetHitResultUnderCursorbyChannel "TraceTypeQuery1" true))
  (bind _asplayer_character (Utilities|Casting|CastToPlayerCharacter (Pawn|GetControlledPawn)))
  (if _returnvalue
    (Transformation|SetActorRotation _asplayer_character (Math|Rotator|MakeRotator 0.0 0.0 (.yaw (Math|Conversions|RotationFromXVector (Math|Vector|GetUnitDirection(Vector) (Transformation|GetActorLocation _asplayer_character) (.Location (Collision|BreakHitResult _hitresult)))))))))

(event EventAtack
  (Utilities|IsValid (Variables|/Game/Blueprints/PlayerCharacter/PlayerCharacter.PlayerCharacter_C|GetArrow1 (stale Input|ActionEvents|InputActionShoot _asplayer_character))
    (:Is%20Valid
      (Game|SpawnActorfromClass "/Game/Blueprints/Actors/Bullet.Bullet_C" (Math|Transform|MakeTransform (.location (Transformation|GetWorldTransform (Variables|/Game/Blueprints/PlayerCharacter/PlayerCharacter.PlayerCharacter_C|GetArrow1 (stale Input|ActionEvents|InputActionShoot _asplayer_character)))) (.rotation (Transformation|GetWorldTransform (Variables|/Game/Blueprints/PlayerCharacter/PlayerCharacter.PlayerCharacter_C|GetArrow1 (stale Input|ActionEvents|InputActionShoot _asplayer_character)))) "0.100000,0.100000,0.100000") "Undefined" 0 (stale Input|ActionEvents|InputActionShoot _asplayer_character)))))

(event Input|ActionEvents|InputActionShoot
  (params (Key :type Key%20Structure))
  (:Pressed
    (bind _asplayer_character (Utilities|Casting|CastToPlayerCharacter (Pawn|GetControlledPawn)))
    (Utilities|IsValid (Variables|/Game/Blueprints/PlayerCharacter/PlayerCharacter.PlayerCharacter_C|GetArrow1 _asplayer_character)
      (:Is%20Valid
        (Variables|/Game/Blueprints/PlayerCharacter/PlayerCharacter.PlayerCharacter_C|Setattacking _asplayer_character true)
        (Utilities|FlowControl|Delay 0.2)
        (Variables|/Game/Blueprints/PlayerCharacter/PlayerCharacter.PlayerCharacter_C|Setattacking _asplayer_character false)))))

(event Input|AxisEvents|InputAxisForwardMove
  (params (AxisValue :type Float%20%28single-precision%29))
  (bind _returnvalue (Pawn|GetControlledPawn))
  (Utilities|IsValid _returnvalue
    (:Is%20Valid
      (Pawn|Input|AddMovementInput _returnvalue (Math|Vector|GetForwardVector (Math|Rotator|MakeRotator 0.0 0.0 (.Yaw (Math|Rotator|BreakRotator (Pawn|GetControlRotation _returnvalue :!class /Script/Engine.Pawn))))) AxisValue false))))

(event Input|AxisEvents|InputAxisRightMove
  (params (AxisValue :type Float%20%28single-precision%29))
  (bind _returnvalue (Pawn|GetControlledPawn))
  (Utilities|IsValid _returnvalue
    (:Is%20Valid
      (Pawn|Input|AddMovementInput _returnvalue (Math|Vector|GetRightVector (Math|Rotator|MakeRotator 0.0 0.0 (.Yaw (Math|Rotator|BreakRotator (Pawn|GetControlRotation _returnvalue :!class /Script/Engine.Pawn))))) AxisValue false))))

(fn ConstructionScript
  (Variables|Default|SetbShowMouseCursor true))