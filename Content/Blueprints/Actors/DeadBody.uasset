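; DeadBody is an actor with a scalable plane that merges with other bodies, damages the player and gradually disappears.
; Each tick, a debug-drawn box trace sized to the plane's scale absorbs equal or smaller DeadBody actors by adding their scale, or applies slight damage to a PlayerCharacter.
; A Tick-driven Delay shrinks the plane proportionally every half second, destroying the actor once it becomes tiny.
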(event EventTick
  (params (DeltaSeconds :type Float%20%28single-precision%29))
  (bind _returnvalue (Transformation|GetActorLocation))
  (bind _plane (Variables|Default|GetPlane))
  (bind _plane_2 (Variables|Default|GetPlane))
  (bind _plane_3 (Variables|Default|GetPlane))
  (bind _returnvalue_2 (Transformation|GetWorldScale _plane_2))
  (bind _returnvalue_3 (Transformation|GetWorldScale _plane_3))
  (bind _returnvalue_4 (Transformation|GetWorldScale _plane))
  (bind _returnvalue_5 (* (.z _returnvalue_2) 5e+01))
  (Utilities|FlowControl|Sequence
    (:then_0
      (Variables|Default|SetSpeedWAGON (* (.x _returnvalue_3) 0.02)))
    (:then_1
      (bind (_outhit _returnvalue_6) (Class|KismetSystemLibrary|BoxTraceSingleforObjects _returnvalue _returnvalue (Math|Vector|MakeVector _returnvalue_5 _returnvalue_5 _returnvalue_5) (Transformation|GetActorRotation) (Utilities|Array|MakeArray "ObjectTypeQuery9" "ObjectTypeQuery7") false (Utilities|Array|MakeArray self) "ForOneFrame" true))
      (if _returnvalue_6
        (bind _asdead_body (Utilities|Casting|CastToDeadBody (.HitActor (Collision|BreakHitResult _outhit)))
          (:then
            (if (>= (.x _returnvalue_4) (.x (Transformation|GetWorldScale (Variables|DeadBody_C|GetPlane _asdead_body))))
              (Transformation|SetWorldScale3D _plane (+ (Math|Vector|MakeVector (.x (Transformation|GetWorldScale (Variables|DeadBody_C|GetPlane _asdead_body))) (.y (Transformation|GetWorldScale (Variables|DeadBody_C|GetPlane _asdead_body))) (.z (Transformation|GetWorldScale (Variables|DeadBody_C|GetPlane _asdead_body)))) (Math|Vector|MakeVector (.x _returnvalue_4) (.y _returnvalue_4) (.z _returnvalue_4))))
              (Actor|DestroyActor _asdead_body)))
          (:CastFailed
            (bind _asplayer_character (Utilities|Casting|CastToPlayerCharacter (.HitActor (Collision|BreakHitResult _outhit))))
            (Game|Damage|ApplyDamage _asplayer_character 0.1 0 0)))))
    (:then_2
      (Utilities|FlowControl|Delay 0.5)
      (Transformation|SetWorldScale3D _plane_3 (Math|Vector|MakeVector (- (.x _returnvalue_3) (Variables|Default|GetSpeedWAGON)) (- (.y _returnvalue_3) (Variables|Default|GetSpeedWAGON)) (- (.z _returnvalue_3) (Variables|Default|GetSpeedWAGON))))
      (if (<= (.x _returnvalue_3) 0.1)
        (Actor|DestroyActor)))))

(event EventDestroyed)

(fn ConstructionScript)