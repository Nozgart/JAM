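; Spawner actor that spawns a requested number of EnemyCharacterFather enemies at its own transform.
; The SpawnEnemy event stores the count in NumOfEnemy, then a while loop spawns and decrements until it reaches zero, with no delay between spawns.
; A one-second delayed respawn branch and a MainGameMode cast are left unused, and BeginPlay, Tick and the construction script are empty.
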(event Custom|SpawnEnemy
  (params (NumOfEnemy :type Integer))
  (Variables|Default|SetNumOfEnemy NumOfEnemy)
  (while (> (Variables|Default|GetNumOfEnemy) 0)
    (Game|SpawnActorfromClass "/Game/Blueprints/EnemyCharacter/EnemyCharacterFather.EnemyCharacterFather_C" (Transformation|GetActorTransform) "Undefined" 0 0)
    (Math|Integer|DecrementInt (Variables|Default|GetNumOfEnemy))))

(event EventBeginPlay)

(event Collision|EventActorBeginOverlap
  (params (OtherActor :type Actor%20Object%20Reference)))

(event EventTick
  (params (DeltaSeconds :type Float%20%28single-precision%29)))

(fn ConstructionScript)