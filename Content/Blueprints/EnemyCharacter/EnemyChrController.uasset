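; AI controller for enemy characters that sends its pawn after the player character and destroys the pawn when the move succeeds.
; Tick issues the AI move request toward the first player's character every frame.
; Possession stores the spawn location, and a WhereToGo event repeats the chase logic for a given target when its state string is Player.
; Rotating sphere-trace detection, which would feed WhereToGo, plus return-to-spawn and stop-movement logic are disconnected and never run.
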(event Custom|WhereToGo
  (params (TargetChr :type Player%20Character%20Object%20Reference))
  (bind _returnvalue (Pawn|GetControlledPawn))
  (switch string (Variables|Default|GetWhereToGoString)
    (:Player
      (AI|AIMoveTo _returnvalue "0, 0, 0" TargetChr 2e+01 false
        (:OnSuccess
          (Actor|DestroyActor _returnvalue))))))

(event EventTick
  (params (DeltaSeconds :type Float%20%28single-precision%29))
  (bind _returnvalue (Pawn|GetControlledPawn))
  (AI|AIMoveTo _returnvalue "0, 0, 0" (Game|GetPlayerCharacter 0) 2e+01 false
    (:OnSuccess
      (Actor|DestroyActor _returnvalue))))

(event EventOnPossess
  (params (PossessedPawn :type Pawn%20Object%20Reference))
  (Variables|Default|SetSpawnLocation (Transformation|GetActorLocation (Pawn|GetControlledPawn))))

(fn ConstructionScript)